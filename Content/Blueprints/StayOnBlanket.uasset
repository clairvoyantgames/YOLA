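; StayOnBlanket is a boundary trigger that fails the player when the ant leaves its box while the ladybug is still alive.
; On Box1 end overlap with MyAnt, it checks the IsDead flag on the referenced BP_LadyBug.
; If the ladybug is not dead, it pauses the player through MyPlayerController, prints a taunt and calls Dead on BP_MyHud.
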(event OnComponentEndOverlap(Box1)
  (params (OtherActor :type Actor%20Object%20Reference) (OtherComp :type Primitive%20Component%20Object%20Reference) (OtherBodyIndex :type Integer))
  (Utilities|Casting|CastToMyAnt OtherActor)
  (bind _asmyplayercontroller (Utilities|Casting|CastToMyPlayerController (Game|GetPlayerController 0)))
  (bind _asbp_ladybug_c (Utilities|Casting|CastToBP_LadyBug (Variables|Default|Getludybug)))
  (if (not (Variables|/Script/YOLA.Creature|GetbIsDead _asbp_ladybug_c))
    (Class|MyPlayerController|PausePlayer _asmyplayercontroller)
    (Development|PrintString "You Suck Nub")
    (bind _asbp_myhud_c (Utilities|Casting|CastToBP_MyHud (HUD|GetHUD (Game|GetPlayerController 0))))
    (Default|Dead _asbp_myhud_c)))

(fn ConstructionScript)