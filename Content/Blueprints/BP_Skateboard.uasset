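; BP_Skateboard is a rideable platform that shuttles the player ant back and forth along the X axis.
; An overlap with BP_MyAnt while idle triggers a FlipFlop that alternates a fast MoveComponentTo of the root by a fixed distance in either direction.
; While IsMoving is set, Tick snaps player pawn 0 to the board's location without sweep, and further overlaps are ignored.
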(event EventActorBeginOverlap
  (params (OtherActor :type Actor%20Object%20Reference))
  (bind _returnvalue (Transformation|GetActorLocation))
  (bind _returnvalue_2 (Transformation|GetActorLocation))
  (bind (_x _y _z) (Math|Vector|BreakVector _returnvalue))
  (bind (_x_2 _y_2 _z_2) (Math|Vector|BreakVector _returnvalue_2))
  (Utilities|Casting|CastToBP_MyAnt OtherActor)
  (if (not (Variables|Default|GetisMoving))
    (Utilities|FlowControl|FlipFlop
      (:A
        (Variables|Default|SetisMoving true)
        (Components|MoveComponentTo (VehicleSound|GetRootComponent) (Math|Vector|MakeVector (+ _x_2 -3.5e+03) _y_2 _z_2) (Transformation|GetActorRotation) false false 0.6)
        (Variables|Default|SetisMoving false))
      (:B
        (Variables|Default|SetisMoving true)
        (Components|MoveComponentTo (VehicleSound|GetRootComponent) (Math|Vector|MakeVector (+ _x 3.5e+03) _y _z) (Transformation|GetActorRotation) false false 0.6)
        (Variables|Default|SetisMoving false)))))

(event EventTick
  (params (DeltaSeconds :type Float%20%28single-precision%29))
  (if (Variables|Default|GetisMoving)
    (Transformation|SetActorLocation (Game|Player|GetPlayerPawn 0) (Transformation|GetActorLocation) false)))

(fn ConstructionScript)