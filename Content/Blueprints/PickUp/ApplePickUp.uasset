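; ApplePickUp is an apple pickup Blueprint that taunts an ant player who is too weak for it.
; When a MyAnt overlaps Box1 with PowerLevel below PowerLevelRequired, it shows a random insult on TextRender1, hidden again on end overlap.
; The random range of four leaves the last two of six lines unreachable.
; This graph has no logic for a sufficiently strong ant.
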(event OnComponentBeginOverlap(Box1)
  (params (OtherActor :type Actor%20Object%20Reference) (OtherComp :type Primitive%20Component%20Object%20Reference) (OtherBodyIndex :type Integer) (bFromSweep :type Boolean) (SweepResult :type Hit%20Result%20Structure%20%28by%20ref%29))
  (bind _asmyant (Utilities|Casting|CastToMyAnt OtherActor))
  (Math|Float|CompareFloat (Variables|/Script/YOLA.MyAnt|GetPowerLevel _asmyant) (Variables|Default|GetPowerLevelRequired)
    (:<
      (switch int (Math|Random|RandomInteger 4)
        (:0
          (Variables|Default|SetNewVar "Bro, Do you even?"))
        (:1
          (Variables|Default|SetNewVar "Too weak, eat something"))
        (:2
          (Variables|Default|SetNewVar "Not with those arms"))
        (:3
          (Variables|Default|SetNewVar "Not 'Mirin"))
        (:4
          (Variables|Default|SetNewVar "Eat much?"))
        (:5
          (Variables|Default|SetNewVar "Do you even Ant?")))
      (Rendering|Components|TextRender|SetText (Variables|Default|GetTextRender1) (Variables|Default|GetNewVar))
      (Rendering|SetVisibility (Variables|Default|GetTextRender1) true false))))

(event OnComponentEndOverlap(Box1)
  (params (OtherActor :type Actor%20Object%20Reference) (OtherComp :type Primitive%20Component%20Object%20Reference) (OtherBodyIndex :type Integer))
  (bind _textrender1 (Variables|Default|GetTextRender1))
  (Utilities|Casting|CastToMyAnt OtherActor)
  (if (Rendering|IsVisible _textrender1)
    (Rendering|SetVisibility _textrender1 false false)))

(fn ConstructionScript)