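; BP_Grasshoppa is an actor that moves to one of four target references, Target1 to Target4, selected by an index passed to its Move event.
; Move calls StopAll to halt all four timelines, then plays the chosen one from the start.
; Each timeline lerps from the actor's current location, rather than a cached start, toward its target without sweeping, so the track's alpha compounds every update.
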(event Custom|StopAll
  (Utilities|FlowControl|Sequence
    (:then_0
      (bind _newtrack_0 (Timeline|Timeline_0 Stop)
        (:Update
          (Transformation|SetActorLocation (Math|Vector|Lerp(Vector) (Transformation|GetActorLocation) (Transformation|GetActorLocation (Variables|Default|GetTarget1)) _newtrack_0) false))))
    (:then_1
      (bind _newtrack_1 (Timeline|Timeline_1 Stop)
        (:Update
          (Transformation|SetActorLocation (Math|Vector|Lerp(Vector) (Transformation|GetActorLocation) (Transformation|GetActorLocation (Variables|Default|GetTarget2)) _newtrack_1) false))))
    (:then_2
      (bind _newtrack_2 (Timeline|Timeline_2 Stop)
        (:Update
          (Transformation|SetActorLocation (Math|Vector|Lerp(Vector) (Transformation|GetActorLocation) (Transformation|GetActorLocation (Variables|Default|GetTarget3)) _newtrack_2) false))))
    (:then_3
      (bind _newtrack_3 (Timeline|Timeline_3 Stop)
        (:Update
          (Transformation|SetActorLocation (Math|Vector|Lerp(Vector) (Transformation|GetActorLocation) (Transformation|GetActorLocation (Variables|Default|GetTarget4)) _newtrack_3) false))))))

(event Custom|Move
  (params (NewParam :type Integer))
  (switch int NewParam
    (:0
      (CallFunction|StopAll)
      (bind _newtrack_0 (Timeline|Timeline_0 PlayFromStart)
        (:Update
          (Transformation|SetActorLocation (Math|Vector|Lerp(Vector) (Transformation|GetActorLocation) (Transformation|GetActorLocation (Variables|Default|GetTarget1)) _newtrack_0) false))))
    (:1
      (CallFunction|StopAll)
      (bind _newtrack_1 (Timeline|Timeline_1 PlayFromStart)
        (:Update
          (Transformation|SetActorLocation (Math|Vector|Lerp(Vector) (Transformation|GetActorLocation) (Transformation|GetActorLocation (Variables|Default|GetTarget2)) _newtrack_1) false))))
    (:2
      (CallFunction|StopAll)
      (bind _newtrack_2 (Timeline|Timeline_2 PlayFromStart)
        (:Update
          (Transformation|SetActorLocation (Math|Vector|Lerp(Vector) (Transformation|GetActorLocation) (Transformation|GetActorLocation (Variables|Default|GetTarget3)) _newtrack_2) false))))
    (:3
      (CallFunction|StopAll)
      (bind _newtrack_3 (Timeline|Timeline_3 PlayFromStart)
        (:Update
          (Transformation|SetActorLocation (Math|Vector|Lerp(Vector) (Transformation|GetActorLocation) (Transformation|GetActorLocation (Variables|Default|GetTarget4)) _newtrack_3) false))))))

(fn ConstructionScript)