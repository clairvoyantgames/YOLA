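; BP_StickPickUp is a stick pickup that reports its horizontal distance to another stick while it is picked up.
; On BeginPlay it searches all stick pickups and stores one other than itself as OtherStick, with the last match winning.
; Each Tick while picked up, it prints that distance on screen as debug output, with no further gameplay logic.
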(event EventBeginPlay
  (bind _outactors (Actor|GetAllActorsOfClass "BP_StickPickup_C"))
  (for _array_element _outactors
    (if (!= _array_element self)
      (bind _asbp_stickpickup_c (Utilities|Casting|CastToBP_StickPickup _array_element))
      (Variables|Default|SetOtherStick _asbp_stickpickup_c))))

(event EventTick
  (params (DeltaSeconds :type Float%20%28single-precision%29))
  (if (Class|PickUp|IsPickedUp)
    (bind _returnvalue (Transformation|GetHorizontalDistanceTo self (Variables|Default|GetOtherStick)))
    (Development|PrintString (Utilities|String|ToString(Float) _returnvalue))))

(fn ConstructionScript)